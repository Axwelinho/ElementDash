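; Water-themed ground tile that has the game mode add another tile when BP_Character overlaps its Box trigger.
; On BeginPlay a random roll can enable Obstacle2, a laser obstacle slid along local Y by a Timeline, or neither.
; ElementCollider overlaps set the game mode's TerrainElement to Water.
; GetArrowTransform exposes the Arrow component's world transform.
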(event `self.ReceiveBeginPlay`
  (bind _obstacle2 (`self.Obstacle2`))
  (bind _obstacle_laser1 (`self.Obstacle_Laser1`))
  (switch `int` (`KismetMathLibrary.RandomIntegerInRange` 0 3)
    (:`0`
      (`SceneComponent.SetVisibility` _obstacle2 true false)
      (`PrimitiveComponent.SetCollisionEnabled` _obstacle2 "QueryAndProbe")
      (`ActorComponent.SetComponentTickEnabled` _obstacle2 true))
    (:`1`
      (`SceneComponent.SetVisibility` _obstacle_laser1 true false)
      (`PrimitiveComponent.SetCollisionEnabled` _obstacle_laser1 "QueryAndProbe")
      (`ActorComponent.SetComponentTickEnabled` _obstacle_laser1 true)
      (bind (_direction _lasermovement) (`Timeline|Timeline`)
        (:`Update`
          (`SceneComponent.K2_AddLocalOffset` (`self.Obstacle_Laser1`) (`KismetMathLibrary.MakeVector` 0.0 _lasermovement) false false))))))

(event `self.Box.OnComponentBeginOverlap`
  (params (OverlappedComponent :type "PrimitiveComponent Object Reference") (OtherActor :type "Actor Object Reference") (OtherComp :type "PrimitiveComponent Object Reference") (OtherBodyIndex :type Integer) (bFromSweep :type Boolean) (SweepResult :type "HitResult Structure (by ref)"))
  (cast `/Game/ThirdPerson/Player/BP_Character` OtherActor)
  (bind _asbp_third_person_game_mode (cast `/Game/ThirdPerson/Blueprints/BP_ThirdPersonGameMode` (`GameplayStatics.GetGameMode`)))
  (`/Game/ThirdPerson/Blueprints/BP_ThirdPersonGameMode.AddGroundTile` _asbp_third_person_game_mode)
  (`KismetSystemLibrary.Delay` 0.2))

(event `self.ElementCollider.OnComponentBeginOverlap`
  (params (OverlappedComponent :type "PrimitiveComponent Object Reference") (OtherActor :type "Actor Object Reference") (OtherComp :type "PrimitiveComponent Object Reference") (OtherBodyIndex :type Integer) (bFromSweep :type Boolean) (SweepResult :type "HitResult Structure (by ref)"))
  (bind _asbp_third_person_game_mode (cast `/Game/ThirdPerson/Blueprints/BP_ThirdPersonGameMode` (`GameplayStatics.GetGameMode`)))
  (set `/Game/ThirdPerson/Blueprints/BP_ThirdPersonGameMode.TerrainElement` "Water" _asbp_third_person_game_mode))

(fn `GetArrowTransform`
  (returns (ArrowTransform :type "Transform Structure"))
  (return (`SceneComponent.K2_GetComponentToWorld` (`self.Arrow`))))

(fn `UserConstructionScript`)