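; Wind-element ground tile for a runner-style track that extends as the character advances.
; On BeginPlay a random roll leaves it plain or adds child actors at fifteen arrow markers, sometimes also enabling Obstacle4.
; A character overlapping Box makes BP_ThirdPersonGameMode add another tile, while any ElementCollider overlap sets its TerrainElement to Wind.
; GetArrowTransform exposes the main Arrow's world transform.
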(event `self.ReceiveBeginPlay`
  (bind _obstacle4 (`self.Obstacle4`))
  (bind _array (`|MakeArray` (`SceneComponent.GetRelativeTransform` (`self.Arrow2`)) (`SceneComponent.GetRelativeTransform` (`self.Arrow3`)) (`SceneComponent.GetRelativeTransform` (`self.Arrow4`)) (`SceneComponent.GetRelativeTransform` (`self.Arrow5`)) (`SceneComponent.GetRelativeTransform` (`self.Arrow6`)) (`SceneComponent.GetRelativeTransform` (`self.Arrow7`)) (`SceneComponent.GetRelativeTransform` (`self.Arrow8`)) (`SceneComponent.GetRelativeTransform` (`self.Arrow9`)) (`SceneComponent.GetRelativeTransform` (`self.Arrow10`)) (`SceneComponent.GetRelativeTransform` (`self.Arrow11`)) (`SceneComponent.GetRelativeTransform` (`self.Arrow12`)) (`SceneComponent.GetRelativeTransform` (`self.Arrow13`)) (`SceneComponent.GetRelativeTransform` (`self.Arrow14`)) (`SceneComponent.GetRelativeTransform` (`self.Arrow15`)) (`SceneComponent.GetRelativeTransform` (`self.Arrow16`))))
  (bind _array_2 (`|MakeArray` (`SceneComponent.GetRelativeTransform` (`self.Arrow2`)) (`SceneComponent.GetRelativeTransform` (`self.Arrow3`)) (`SceneComponent.GetRelativeTransform` (`self.Arrow4`)) (`SceneComponent.GetRelativeTransform` (`self.Arrow5`)) (`SceneComponent.GetRelativeTransform` (`self.Arrow6`)) (`SceneComponent.GetRelativeTransform` (`self.Arrow7`)) (`SceneComponent.GetRelativeTransform` (`self.Arrow8`)) (`SceneComponent.GetRelativeTransform` (`self.Arrow9`)) (`SceneComponent.GetRelativeTransform` (`self.Arrow10`)) (`SceneComponent.GetRelativeTransform` (`self.Arrow11`)) (`SceneComponent.GetRelativeTransform` (`self.Arrow12`)) (`SceneComponent.GetRelativeTransform` (`self.Arrow13`)) (`SceneComponent.GetRelativeTransform` (`self.Arrow14`)) (`SceneComponent.GetRelativeTransform` (`self.Arrow15`)) (`SceneComponent.GetRelativeTransform` (`self.Arrow16`))))
  (switch `int` (`KismetMathLibrary.RandomIntegerInRange` 0 3)
    (:`0`
      (`|ExecutionSequence`
        (:`then_0`
          (for (_ _array_index) _array_2
            (`AddComponent|NODE_AddChildActorComponent-1` :`RelativeTransform` (`|GetArrayItem` _array_2 _array_index))))))
    (:`2`
      (`SceneComponent.SetVisibility` _obstacle4 true false)
      (`PrimitiveComponent.SetCollisionEnabled` _obstacle4 "QueryAndProbe")
      (`ActorComponent.SetComponentTickEnabled` _obstacle4 true)
      (for (_ _array_index_2) _array
        (`AddComponent|NODE_AddChildActorComponent-0` :`RelativeTransform` (`|GetArrayItem` _array _array_index_2))))))

(event `self.Box.OnComponentBeginOverlap`
  (params (OverlappedComponent :type "PrimitiveComponent Object Reference") (OtherActor :type "Actor Object Reference") (OtherComp :type "PrimitiveComponent Object Reference") (OtherBodyIndex :type Integer) (bFromSweep :type Boolean) (SweepResult :type "HitResult Structure (by ref)"))
  (cast `/Game/ThirdPerson/Player/BP_Character` OtherActor)
  (bind _asbp_third_person_game_mode (cast `/Game/ThirdPerson/Blueprints/BP_ThirdPersonGameMode` (`GameplayStatics.GetGameMode`)))
  (`/Game/ThirdPerson/Blueprints/BP_ThirdPersonGameMode.AddGroundTile` _asbp_third_person_game_mode)
  (`KismetSystemLibrary.Delay` 0.2))

(event `self.ElementCollider.OnComponentBeginOverlap`
  (params (OverlappedComponent :type "PrimitiveComponent Object Reference") (OtherActor :type "Actor Object Reference") (OtherComp :type "PrimitiveComponent Object Reference") (OtherBodyIndex :type Integer) (bFromSweep :type Boolean) (SweepResult :type "HitResult Structure (by ref)"))
  (bind _asbp_third_person_game_mode (cast `/Game/ThirdPerson/Blueprints/BP_ThirdPersonGameMode` (`GameplayStatics.GetGameMode`)))
  (set `/Game/ThirdPerson/Blueprints/BP_ThirdPersonGameMode.TerrainElement` "Wind" _asbp_third_person_game_mode))

(fn `GetArrowTransform`
  (returns (ArrowTransform :type "Transform Structure"))
  (return (`SceneComponent.K2_GetComponentToWorld` (`self.Arrow`))))

(fn `UserConstructionScript`)